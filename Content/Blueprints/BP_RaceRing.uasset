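; Race ring checkpoint actor that a BP_Butterfly passes through.
; It starts hidden with box collision off, with separate events to reveal or hide it.
; Activate and deactivate events set the active flag, swap the frame material and toggle query-only box collision.
; When a butterfly overlaps the active ring, it calls OnRingPassed on that butterfly's MyMushroom, passing the butterfly along.
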(event `self.ReceiveBeginPlay`
  (`self.SetActorHiddenInGame` true)
  (`PrimitiveComponent.SetCollisionEnabled` (`self.Box`) "NoCollision"))

(event `ActivateRing`
  (set `self.IsActive` true)
  (`PrimitiveComponent.SetMaterial` (`self.Cube_002`) 0 "/Game/Materials/FrameActive.FrameActive")
  (`PrimitiveComponent.SetCollisionEnabled` (`self.Box`) "QueryOnly"))

(event `Event Reveal Ring`
  (`self.SetActorHiddenInGame` false))

(event `DeactivateRing`
  (set `self.IsActive` false)
  (`PrimitiveComponent.SetMaterial` (`self.Cube_002`) 0 "/Game/Materials/Frame.Frame")
  (`PrimitiveComponent.SetCollisionEnabled` (`self.Box`) "NoCollision"))

(event `Event Hide Ring`
  (`self.SetActorHiddenInGame` true))

(event `self.Box.OnComponentBeginOverlap`
  (params (OverlappedComponent :type "PrimitiveComponent Object Reference") (OtherActor :type "Actor Object Reference") (OtherComp :type "PrimitiveComponent Object Reference") (OtherBodyIndex :type Integer) (bFromSweep :type Boolean) (SweepResult :type "HitResult Structure (by ref)"))
  (bind _asbp_butterfly (cast `/Game/Blueprints/BP_Butterfly` OtherActor))
  (if (`self.IsActive`)
    (`/Game/C++Blueprints/BP_MotherMushroom.OnRingPassed` (`/Game/Blueprints/BP_Butterfly.MyMushroom` _asbp_butterfly) _asbp_butterfly)))

(fn `UserConstructionScript`)