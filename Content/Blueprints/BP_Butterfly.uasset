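; BP_Butterfly is a ship that the first-person player can board and leave through interaction and input.
; Boarding and leaving notify BP_FirstPersonCharacter, gated by its CanSwitchControl flag with a short delay to prevent rapid switching.
; It creates a WB_ButterflyPanel widget on BeginPlay, forwards Scan, Radio and Log inputs to it, and removes it from its parent on leaving.
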(event `self.ReceiveBeginPlay`
  ; Get Player
  (bind _returnvalue (`|CreateWidget` "/Game/UI/WB_ButterflyPanel.WB_ButterflyPanel_C"))
  (set `self.ButterflyUI_Ref` _returnvalue)
  (bind _asbp_first_person_character (cast `/Game/FirstPerson/Blueprints/BP_FirstPersonCharacter` (`GameplayStatics.GetPlayerCharacter` 0)))
  (set `self.Player` _asbp_first_person_character)
  (set `self.ShipStaticMesh` (`self.Cube`)))

(event `/Game/Blueprints/BI_Interactable.Interact`
  (bind _player (`self.Player`))
  (bind _player_2 (`self.Player`))
  ; Player interact with ship
  (if (and (not (`self.OnShipOccupied`)) (`/Game/FirstPerson/Blueprints/BP_FirstPersonCharacter.bCanSwitchControl` _player_2))
    (set `self.OnShipOccupied` true)
    (set `/Game/FirstPerson/Blueprints/BP_FirstPersonCharacter.bCanSwitchControl` false _player_2)
    (set `/Game/FirstPerson/Blueprints/BP_FirstPersonCharacter.CurrentShip` self _player)
    (`/Game/FirstPerson/Blueprints/BP_FirstPersonCharacter.OnShipOccupied` _player)
    (`KismetSystemLibrary.Delay` 1.0)
    (set `/Game/FirstPerson/Blueprints/BP_FirstPersonCharacter.bCanSwitchControl` true _player_2)))

(event `EnhancedInput|/Game/Input/Actions/IA_LeaveShip`
  (params (ActionValue :type Boolean) (ElapsedSeconds :type "Float (double-precision)") (TriggeredSeconds :type "Float (double-precision)") (InputAction :type "InputAction Object Reference" :default "/Game/Input/Actions/IA_LeaveShip.IA_LeaveShip"))
  (bind _player (`self.Player`))
  ; Leave ship
  (:`Started`
    (if (`/Game/FirstPerson/Blueprints/BP_FirstPersonCharacter.bCanSwitchControl` _player)
      (set `/Game/FirstPerson/Blueprints/BP_FirstPersonCharacter.bCanSwitchControl` false _player)
      (`Widget.RemoveFromParent` (`self.ButterflyUI_Ref`))
      (`/Game/FirstPerson/Blueprints/BP_FirstPersonCharacter.OnShipLeave` _player)
      (`KismetSystemLibrary.Delay` 1.0)
      (set `/Game/FirstPerson/Blueprints/BP_FirstPersonCharacter.bCanSwitchControl` true _player))))

(event `OnShipUnoccupied`
  ; Set ship unoccupied
  (set `self.OnShipOccupied` false)
  (set `/Game/FirstPerson/Blueprints/BP_FirstPersonCharacter.CurrentShip` null (`self.Player`)))

(event `EnhancedInput|/Game/Input/Actions/IA_Scan`
  (params (ActionValue :type Boolean) (ElapsedSeconds :type "Float (double-precision)") (TriggeredSeconds :type "Float (double-precision)") (InputAction :type "InputAction Object Reference" :default "/Game/Input/Actions/IA_Scan.IA_Scan"))
  (:`Started`
    (bind _butterflyui_ref (`self.ButterflyUI_Ref`)
      (:`then`
        (`/Game/UI/WB_ButterflyPanel.Action_Scan` _butterflyui_ref))
      (:`else`))))

(event `EnhancedInput|/Game/Input/Actions/IA_Radio`
  (params (ActionValue :type Boolean) (ElapsedSeconds :type "Float (double-precision)") (TriggeredSeconds :type "Float (double-precision)") (InputAction :type "InputAction Object Reference" :default "/Game/Input/Actions/IA_Radio.IA_Radio"))
  (:`Started`
    (bind _butterflyui_ref (`self.ButterflyUI_Ref`)
      (:`then`
        (`/Game/UI/WB_ButterflyPanel.Action_Radio` _butterflyui_ref))
      (:`else`))))

(event `EnhancedInput|/Game/Input/Actions/IA_Log`
  (params (ActionValue :type Boolean) (ElapsedSeconds :type "Float (double-precision)") (TriggeredSeconds :type "Float (double-precision)") (InputAction :type "InputAction Object Reference" :default "/Game/Input/Actions/IA_Log.IA_Log"))
  (:`Started`
    (bind _butterflyui_ref (`self.ButterflyUI_Ref`)
      (:`then`
        (`/Game/UI/WB_ButterflyPanel.Action_Log` _butterflyui_ref))
      (:`else`))))

(fn `UserConstructionScript`)