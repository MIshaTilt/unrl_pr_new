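; BP_Campfire is a campfire actor that appears as built once a resource is added to it.
; It hides its Log1 and Cone components, with their children, on BeginPlay.
; GetRequiredResources reports a fixed resource type and amount as the cost.
; TryAddResource reveals both components and always returns true, without checking the type or amount passed in.
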(event `self.ReceiveBeginPlay`
  (`SceneComponent.SetVisibility` (`self.Log-1`) false true)
  (`SceneComponent.SetVisibility` (`self.Cone`) false true))

(fn `GetRequiredResources`
  (returns (ResourceType :type "/Game/Blueprints/E_ResourceType Enum") (Amount :type Integer))
  (return "NewEnumerator1" 4))

(fn `TryAddResource`
  (params (ResourceType :type "/Game/Blueprints/E_ResourceType Enum" :default "NewEnumerator0") (Amount :type Integer))
  (returns (WasAccepted :type Boolean))
  (`SceneComponent.SetVisibility` (`self.Log-1`) true true)
  (`SceneComponent.SetVisibility` (`self.Cone`) true true)
  (return true))

(fn `UserConstructionScript`)