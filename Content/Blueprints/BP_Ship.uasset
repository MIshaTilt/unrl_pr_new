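; BP_Ship is a ship that the first-person player character can board and leave through interaction.
; On BeginPlay it caches the player character and stores its Cube component as the ship mesh.
; Interacting while unoccupied marks the ship occupied, sets it as the player's CurrentShip and notifies the player.
; The leave input only calls the player's OnShipLeave; a separate OnShipUnoccupied event clears the occupied flag and CurrentShip.
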(event `self.ReceiveBeginPlay`
  ; Get Player
  (bind _asbp_first_person_character (cast `/Game/FirstPerson/Blueprints/BP_FirstPersonCharacter` (`GameplayStatics.GetPlayerCharacter` 0)))
  (set `self.Player` _asbp_first_person_character)
  (set `self.ShipStaticMesh` (`self.Cube`)))

(event `/Game/Blueprints/BI_Interactable.Interact`
  (bind _player (`self.Player`))
  ; Player interact with ship
  (if (not (`self.OnShipOccupied`))
    (set `self.OnShipOccupied` true)
    (set `/Game/FirstPerson/Blueprints/BP_FirstPersonCharacter.CurrentShip` self _player)
    (`/Game/FirstPerson/Blueprints/BP_FirstPersonCharacter.OnShipOccupied` _player)))

(event `EnhancedInput|/Game/Input/Actions/IA_LeaveShip`
  (params (ActionValue :type Boolean) (ElapsedSeconds :type "Float (double-precision)") (TriggeredSeconds :type "Float (double-precision)") (InputAction :type "InputAction Object Reference" :default "/Game/Input/Actions/IA_LeaveShip.IA_LeaveShip"))
  ; Leave ship
  (:`Started`
    (`/Game/FirstPerson/Blueprints/BP_FirstPersonCharacter.OnShipLeave` (`self.Player`))))

(event `OnShipUnoccupied`
  ; Set ship unoccupied
  (set `self.OnShipOccupied` false)
  (set `/Game/FirstPerson/Blueprints/BP_FirstPersonCharacter.CurrentShip` null (`self.Player`)))

(fn `UserConstructionScript`)