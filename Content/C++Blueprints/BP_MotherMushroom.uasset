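; Mother mushroom actor that takes spores, spawns a player butterfly and hosts its timed ring race.
; State changes toggle Visibility collision on the mesh and interact proxy to control interaction.
; Race prep reveals RaceRings and debug-draws a spline through them, then rings activate in sequence.
; Finishing saves the best time per TrackID to SG_RaceRecords, updates the HUD, then exits the butterfly and hides rings.
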(event `BuildTrajectory`
  (bind _trajectoryspline (`self.TrajectorySpline`))
  (`SplineComponent.ClearSplinePoints` _trajectoryspline true)
  (for (_array_element _array_index) (`self.RaceRings`)
    (`KismetSystemLibrary.PrintString` (`KismetSystemLibrary.GetDisplayName` _array_element))
    (`SplineComponent.AddSplinePoint` _trajectoryspline (`self.K2_GetActorLocation` _array_element) "World" true)
    (`SplineComponent.SetTangentAtSplinePoint` _trajectoryspline _array_index (* (`self.GetActorForwardVector` _array_element) (`self.Tension`)) "World" true)))

(event `StartSpawnSequence`
  (`KismetSystemLibrary.PrintString` "Interact")
  (bind _returnvalue (`self.SpawnButterfly`))
  (bind _asbp_butterfly (cast `/Game/Blueprints/BP_Butterfly` _returnvalue)
    (:`then`
      (set `/Game/Blueprints/BP_Butterfly.MyMushroom` self _asbp_butterfly)
      (`KismetSystemLibrary.PrintString` "УСПЕХ"))
    (:`CastFailed`
      (`KismetSystemLibrary.PrintString` "cast fail on interact"))))

(event `self.ReceiveBeginPlay`
  (`KismetSystemLibrary.PrintString` "1")
  (bind _asbp_mushroom_proxy (cast `/Game/C++Blueprints/BP_MushroomProxy` (`ChildActorComponent.ChildActor` (`self.InteractProxy`))))
  (`PrimitiveComponent.SetCollisionResponseToChannel` (`/Game/C++Blueprints/BP_MushroomProxy.ProxyCollision` _asbp_mushroom_proxy) "ECC_Visibility" "ECR_Ignore"))

(event `self.OnStateChanged`
  (params (NewState :type "EMushroomState Enum" :default "NeedsSpores"))
  (bind _meshcomp (`self.MeshComp`))
  (bind _childactor (`ChildActorComponent.ChildActor` (`self.InteractProxy`)))
  (switch `EMushroomState` NewState
    (:`NeedsSpores`
      (`PrimitiveComponent.SetCollisionResponseToChannel` _meshcomp "ECC_Visibility" "ECR_Block")
      (`KismetSystemLibrary.PrintString` "1")
      (bind _asbp_mushroom_proxy (cast `/Game/C++Blueprints/BP_MushroomProxy` _childactor))
      (`PrimitiveComponent.SetCollisionResponseToChannel` (`/Game/C++Blueprints/BP_MushroomProxy.ProxyCollision` _asbp_mushroom_proxy) "ECC_Visibility" "ECR_Ignore"))
    (:`ReadyToBloom`
      (`PrimitiveComponent.SetCollisionResponseToChannel` _meshcomp "ECC_Visibility" "ECR_Ignore")
      (`KismetSystemLibrary.PrintString` "2")
      (bind _asbp_mushroom_proxy_2 (cast `/Game/C++Blueprints/BP_MushroomProxy` _childactor))
      (`PrimitiveComponent.SetCollisionResponseToChannel` (`/Game/C++Blueprints/BP_MushroomProxy.ProxyCollision` _asbp_mushroom_proxy_2) "ECC_Visibility" "ECR_Block"))
    (:`Symbiosis`
      (`PrimitiveComponent.SetCollisionResponseToChannel` _meshcomp "ECC_Visibility" "ECR_Ignore")
      (`KismetSystemLibrary.PrintString` "3")
      (bind _asbp_mushroom_proxy_3 (cast `/Game/C++Blueprints/BP_MushroomProxy` _childactor))
      (`PrimitiveComponent.SetCollisionResponseToChannel` (`/Game/C++Blueprints/BP_MushroomProxy.ProxyCollision` _asbp_mushroom_proxy_3) "ECC_Visibility" "ECR_Ignore"))))

(event `StartRace`
  (set `self.CurrentRingIndex` 0)
  (`/Game/Blueprints/BP_RaceRing.ActivateRing` (`|GetArrayItem` (`self.RaceRings`)))
  (set `self.RaceStartTime` (`KismetSystemLibrary.GetGameTimeInSeconds`))
  (set `self.IsRaceActive` true)
  (set `self.IsRaceEnded` false))

(event `PrepareRace`
  (for _array_element (`self.RaceRings`)
    (`/Game/Blueprints/BP_RaceRing.Event Reveal Ring` _array_element)
    (`self.BuildTrajectory`)
    (`self.DebugDrawTrajectory`)))

(event `OnRingPassed`
  (params (PassingButterfly :type "/Game/Blueprints/BP_Butterfly Object Reference"))
  (bind _currentringindex (`self.CurrentRingIndex`))
  (`/Game/Blueprints/BP_RaceRing.DeactivateRing` (`|GetArrayItem` (`self.RaceRings`) _currentringindex))
  (bind _output_get (set `self.CurrentRingIndex` (+ _currentringindex 1)))
  (if (>= _output_get (`KismetArrayLibrary.Array_Length` (`self.RaceRings`)))
    (`self.FinishRace` PassingButterfly)
    (else
      (`/Game/Blueprints/BP_RaceRing.ActivateRing` (`|GetArrayItem` (`self.RaceRings`) _output_get)))))

(event `FinishRace`
  (params (FinishedButterfly :type "/Game/Blueprints/BP_Butterfly Object Reference"))
  (bind _activehud (`/Game/Blueprints/BP_Butterfly.ActiveHUD` FinishedButterfly))
  (bind _trackid (`self.TrackID`))
  (bind _returnvalue (- (`KismetSystemLibrary.GetGameTimeInSeconds`) (`self.RaceStartTime`)))
  (`KismetSystemLibrary.PrintString` (`KismetStringLibrary.Concat_StrStr` "ФИНИШ! Ваше время: " (`KismetStringLibrary.Conv_DoubleToString` _returnvalue)))
  (bind _returnvalue_2 (`GameplayStatics.DoesSaveGameExist` "Records"))
  (if _returnvalue_2
    (bind _returnvalue_3 (`GameplayStatics.LoadGameFromSlot` "Records"))
    (bind _assg_race_records (cast `/Game/Blueprints/SG_RaceRecords` _returnvalue_3))
    (bind _output_get (set `self.CurrentSave` _assg_race_records))
    (bind _besttimes (`/Game/Blueprints/SG_RaceRecords.BestTimes` _output_get))
    (bind (_value _returnvalue_4) (`BlueprintMapLibrary.Map_Find` _besttimes _trackid))
    (if _returnvalue_4
      (if (< _value _returnvalue)
        (set `self.IsRaceActive` false)
        (`/Game/UI/WBP_RaceHUD.SetFinalTime` _activehud _returnvalue)
        (else
          (`BlueprintMapLibrary.Map_Add` _besttimes _trackid _returnvalue :!label _label)
          (`GameplayStatics.SaveGameToSlot` (`self.CurrentSave`) "Records")
          (set `self.IsRaceActive` false)
          (set `self.FinalRaceTime` _returnvalue)
          (`/Game/UI/WBP_RaceHUD.SetFinalTime` _activehud _returnvalue)))
      (else
        (goto _label)))
    (else
      (bind _returnvalue_5 (`GameplayStatics.CreateSaveGameObject` "/Game/Blueprints/SG_RaceRecords.SG_RaceRecords_C"))
      (set `self.CurrentSave` _returnvalue_5)
      (goto _label)))
  (`KismetSystemLibrary.Delay` 5.0)
  (`/Game/Blueprints/BP_Butterfly.LeaveButterfly` FinishedButterfly)
  (for _array_element (`self.RaceRings`)
    (`/Game/Blueprints/BP_RaceRing.Event Hide Ring` _array_element)))

(fn `DebugDrawTrajectory`
  (locals (PrevLocation :type "Vector Structure") (StepSize :type "Float (double-precision)" :default 100.0))
  (bind _trajectoryspline (`self.TrajectorySpline`))
  (bind _trajectoryspline_2 (`self.TrajectorySpline`))
  (bind _prevlocation (`local.PrevLocation`))
  (bind _returnvalue (`SplineComponent.GetSplineLength` _trajectoryspline))
  (set `local.PrevLocation` (`SplineComponent.GetLocationAtDistanceAlongSpline` _trajectoryspline 0.0 "World"))
  (for _index (range 1 (+ (`KismetMathLibrary.FTrunc` (/ _returnvalue (`local.StepSize`))) 1))
    (bind _returnvalue_2 (`SplineComponent.GetLocationAtDistanceAlongSpline` _trajectoryspline_2 (* _index (`local.StepSize`)) "World"))
    (`KismetSystemLibrary.DrawDebugLine` _prevlocation _returnvalue_2 (struct :`R` 0.223228 :`G` 0.879623 :`B` 1.0 :`A` 1.0) 9999999.0 10.0)
    (bind _output_get (set `local.PrevLocation` _returnvalue_2))
    (`KismetSystemLibrary.PrintString` (`KismetStringLibrary.Conv_VectorToString` _output_get)))
  (`KismetSystemLibrary.DrawDebugLine` _prevlocation (`SplineComponent.GetLocationAtDistanceAlongSpline` _trajectoryspline_2 _returnvalue "World") (struct :`R` 0.223228 :`G` 0.879623 :`B` 1.0 :`A` 1.0) 999999999.0 10.0))

(fn `GetRequiredResources`
  (returns (ResourceType :type "/Game/Blueprints/E_ResourceType Enum") (Amount :type Integer))
  (return "NewEnumerator2" (`self.GetMissingSpores`)))

(fn `TryAddResource`
  (params (ResourceType :type "/Game/Blueprints/E_ResourceType Enum" :default "NewEnumerator0") (Amount :type Integer))
  (returns (WasAccepted :type Boolean))
  (bind _returnvalue (`self.AddSpores` Amount))
  (return _returnvalue))

(fn `UserConstructionScript`)